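; BP_DamageBall is a hazard ball that costs the player a life when BP_Personaje overlaps its sphere collision.
; A DoOnce-guarded overlap decrements the lives stored in GI_GameInstance, cached at BeginPlay, and refreshes the referenced widget.
; With lives remaining the ball destroys itself.
; Otherwise it triggers game over, hides, and after a short delay resets the lives and reloads Level1.
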(event OnComponentBeginOverlap(SphereCollision)
  (params (OverlappedComponent :type Primitive%20Component%20Object%20Reference) (OtherActor :type Actor%20Object%20Reference) (OtherComp :type Primitive%20Component%20Object%20Reference) (OtherBodyIndex :type Integer) (bFromSweep :type Boolean) (SweepResult :type Hit%20Result%20Structure%20%28by%20ref%29))
  (bind _as_gi_game_instance (Variables|Default|GetAs%20GI%20Game%20Instance))
  ;[0.07062 0.15 0.1021 0.5] Si tocas bolas lrestamos una vida, destruimos la bol y actualizamos widget.
  (Utilities|Casting|CastToBP_Personaje OtherActor)
  (Utilities|FlowControl|DoOnce false
    (:Completed
      (bind _result (Math|Integer|DecrementInt (Variables|/Game/Blueprints/GI_GameInstance.GI_GameInstance_C|GetiLives (Variables|Default|GetAs%20GI%20Game%20Instance)))
        (:%20%20
          (bind _output_get (Variables|/Game/Blueprints/GI_GameInstance.GI_GameInstance_C|SetiLives (Variables|Default|GetAs%20GI%20Game%20Instance) _result))
          (Default|RefreshLives (Variables|/Game/Blueprints/GI_GameInstance.GI_GameInstance_C|GetWidgetReference (Variables|Default|GetAs%20GI%20Game%20Instance)) _output_get)
          (Utilities|FlowControl|Sequence
            (:then_0
              (if (<= _output_get 0)
                (Default|GameOver (Variables|/Game/Blueprints/GI_GameInstance.GI_GameInstance_C|GetWidgetReference _as_gi_game_instance))
                (Rendering|SetActorHiddenInGame true)
                (Utilities|FlowControl|Delay 1.5)
                (Variables|/Game/Blueprints/GI_GameInstance.GI_GameInstance_C|SetiLives _as_gi_game_instance 3)
                (Game|OpenLevel(byName) "Level1")
                (else
                  (Actor|DestroyActor))))))))))

(event EventBeginPlay
  ;[0.01576 0.15 0.06094 0.5] Guardamos instancia a gameinstance
  (bind _asgi_game_instance (Utilities|Casting|CastToGI_GameInstance (Game|GetGameInstance)))
  (Variables|Default|SetAs%20GI%20Game%20Instance _asgi_game_instance))

(fn ConstructionScript)