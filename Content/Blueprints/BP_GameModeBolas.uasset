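; Game mode Blueprint that runs a level countdown and opens Level1 when time runs out.
; On BeginPlay it creates WBP_Display with three lives, adds it to the viewport and passes its reference to the GameInstance through BPI_GameInstance.
; Only if that interface is implemented, a looping timer calls UpdateCountdown every second.
; UpdateCountdown decrements CountdownTime and prints a debug warning at five seconds remaining.
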(event EventBeginPlay
  (bind _returnvalue (Game|GetGameInstance))
  ;[0.007127 0.15 0.03334 0.5] Creamos el widget y guardamos una referencia a el en el GameInstance.
  (bind _returnvalue_2 (UserInterface|CreateWidget "/Game/Blueprints/WBP_Display.WBP_Display_C"))
  (bind _output_get (Variables|Default|SetWidgetRef _returnvalue_2))
  (UserInterface|Viewport|AddtoViewport _output_get 0)
  (if (Utilities|DoesObjectImplementInterface _returnvalue "/Game/Blueprints/BPI_GameInstance.BPI_GameInstance_C")
    (Class|BPIGameInstance|SetRefWidgetFunction(Message) _returnvalue (Variables|Default|GetWidgetRef))
    (Utilities|Time|SetTimerbyFunctionName 0 "UpdateCountdown" 1.0 true)))

(fn ConstructionScript)

(fn UpdateCountdown
  ;[0.15 0.01719 0.03666 0.5] Reglamento de si es 5 segundos antes de acabar avisa. Estaría bien ponerlo en el Widget un timer de cuenta atrás.
  (Math|Integer|DecrementInt (Variables|Default|GetCountdownTime)
    (:%20%20
      (Variables|Default|SetCountdownTime (Variables|Default|GetCountdownTime))
      (if (== (Variables|Default|GetCountdownTime) 5)
        (Development|PrintString "ES IGUAL A 5" true true "(R=0.000000,G=0.660000,B=1.000000,A=1.000000)" 3.0)
        (elif (<= (Variables|Default|GetCountdownTime) 0)
          (Game|OpenLevel(byName) "Level1"))))))