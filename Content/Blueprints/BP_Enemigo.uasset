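; BP_Enemigo is an enemy that patrols target points matching its tag name and reacts to perceiving the player.
; It loops through the points with AI MoveTo and short pauses.
; On sight it chases the player, printing "game over" on arrival.
; When sight is lost it searches the last seen location and a random nearby point without explicitly resuming patrol, while hearing only prints a debug message.
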(event OnTargetPerceptionUpdated(AIPerception)
  (params (Actor :type Actor%20Object%20Reference) (Stimulus :type AI%20Stimulus%20Structure))
  ;[0 0.15 0.06361 0.5] Seguir y luego buscar un rato en el ultimo sitio que te ha visto.
  (if (Actor|ActorHasTag Actor "Player")
    (bind _output_get (Variables|Default|SetStimulus Stimulus))
    (bind _returnvalue (Class|AIPerceptionSystem|GetSenseClassforStimulus _output_get))
    (if (== _returnvalue "/Script/AIModule.AISense_Sight")
      (if (.bsuccessfullysensed (Variables|Default|GetStimulus))
        (AI|AIMoveTo self "0, 0, 0" (Game|GetPlayerCharacter 0) 5.0 false
          (:OnSuccess
            (Development|PrintString "game over" true true "(R=0.000000,G=1.000000,B=0.123647,A=1.000000)")))
        (else
          (bind _output_get_2 (Variables|Default|SetPlayerPosition (.stimuluslocation (Variables|Default|GetStimulus))))
          (AI|AIMoveTo self _output_get_2 0 5.0 false
            (:OnSuccess
              (Utilities|FlowControl|Delay 1.0)
              (AI|AIMoveTo self (.RandomLocation (AI|Navigation|GetRandomReachablePointinRadius (Transformation|GetActorLocation) 5e+02 0 0)) 0 5.0 false
                (:OnSuccess
                  (Development|PrintString "ya he investigado" true true "(R=0.000000,G=1.000000,B=0.123647,A=1.000000)")))))))
      (elif (== _returnvalue "/Script/AIModule.AISense_Hearing")
        (Development|PrintString "HEAR PLAYER" true true "(R=0.938764,G=0.000000,B=1.000000,A=1.000000)")))))

(event Custom|Patrullar
  ;[0.15 0.15 0.15 0.5] Comment
  (if (== (Variables|Default|GetActualTargetPoint) (- (Utilities|Array|Length (Variables|Default|GetTargetPoints)) 1))
    (Variables|Default|SetActualTargetPoint 0)
    (else
      (Variables|Default|SetActualTargetPoint (+ (Variables|Default|GetActualTargetPoint) 1))))
  (AI|AIMoveTo self (Transformation|GetActorLocation (Utilities|Array|Get(acopy) (Variables|Default|GetTargetPoints) (Variables|Default|GetActualTargetPoint))) 0 5.0 false
    (:OnSuccess
      (Utilities|FlowControl|Delay 1.0)
      (CallFunction|Patrullar))))

(event EventBeginPlay
  ;[0 0.15 0.02207 0.5] Seleccionamos todas las target points. Cada target point tiene asignado el nombre del enemigo que deberia tarjetear.
  (bind _outactors (Actor|GetAllActorsOfClasswithTag "/Script/Engine.TargetPoint" (Variables|Default|GetTargetPointName)))
  (Variables|Default|SetTargetPoints _outactors)
  (Utilities|IsValid (Utilities|Array|Get(acopy) (Variables|Default|GetTargetPoints) (Variables|Default|GetActualTargetPoint))
    (:Is%20Valid
      (AI|AIMoveTo self (Transformation|GetActorLocation (Utilities|Array|Get(acopy) (Variables|Default|GetTargetPoints) (Variables|Default|GetActualTargetPoint))) 0 5.0 false
        (:OnSuccess
          (Utilities|FlowControl|Delay 1.0)
          (CallFunction|Patrullar))))))

(fn ConstructionScript)