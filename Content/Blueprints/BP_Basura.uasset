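; BP_Basura is an AI enemy that patrols, investigates and chases the player using AI Perception and AIMoveTo.
; It loops through TargetPoints at BeginPlay, setting a movement speed for each behavior.
; Seeing the player starts a chase that prints "game over" on arrival.
; Lost sight or tagged sounds from the player trigger a move to the stimulus location, then one random nearby move with no return to patrol.
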(event OnTargetPerceptionUpdated(AIPerception)
  (params (Actor :type Actor%20Object%20Reference) (Stimulus :type AI%20Stimulus%20Structure))
  (bind _output_get (Variables|Default|SetStimulus Stimulus))
  (if (Actor|ActorHasTag Actor "Player")
    (bind _returnvalue (Class|AIPerceptionSystem|GetSenseClassforStimulus _output_get))
    (if (== _returnvalue "/Script/AIModule.AISense_Sight")
      (if (.bsuccessfullysensed (Variables|Default|GetStimulus))
        (CallFunction|Perseguir)
        (else
          (Variables|Default|SetPlayerPosition (.stimuluslocation (Variables|Default|GetStimulus)))
          (CallFunction|Investigar)))
      (elif (== _returnvalue "/Script/AIModule.AISense_Hearing")
        (switch name (.tag (Variables|Default|GetStimulus))
          (:PlayerSound
            _)
          (:OtherSound
            _))
        (Variables|Default|SetPlayerPosition (.stimuluslocation (Variables|Default|GetStimulus)))
        (CallFunction|Investigar)))))

(event Custom|Investigar
  (CallFunction|SetIASpeed 0)
  (AI|AIMoveTo self (Variables|Default|GetPlayerPosition) 0 5.0 false
    (:OnSuccess
      (Utilities|FlowControl|Delay 1.0)
      (CallFunction|Explorar))))

(event Custom|Patrol
  (bind _targetpoints (Variables|Default|GetTargetPoints))
  (bind _output (Utilities|Array|Get(acopy) _targetpoints))
  (CallFunction|SetIASpeed)
  (Utilities|IsValid _output
    (:Is%20Valid
      (Variables|Default|SetIndexTargetPoints 0)
      (AI|AIMoveTo self (Transformation|GetActorLocation _output) 0 5.0 false
        (:OnSuccess
          (Utilities|FlowControl|Delay 1.0)
          (CallFunction|NextPoint))))))

(event Custom|Perseguir
  (CallFunction|SetIASpeed 0)
  (AI|AIMoveTo self "0, 0, 0" (Game|GetPlayerCharacter 0) 5.0 false
    (:OnSuccess
      (Development|PrintString "game over" true true "(R=0.000000,G=1.000000,B=0.123647,A=1.000000)"))))

(event Custom|NextPoint
  (if (== (Variables|Default|GetIndexTargetPoints) (- (Utilities|Array|Length (Variables|Default|GetTargetPoints)) 1))
    (Variables|Default|SetIndexTargetPoints 0)
    (else
      (Variables|Default|SetIndexTargetPoints (+ (Variables|Default|GetIndexTargetPoints) 1))))
  (Utilities|IsValid (Utilities|Array|Get(acopy) (Variables|Default|GetTargetPoints) (Variables|Default|GetIndexTargetPoints))
    (:Is%20Valid
      (AI|AIMoveTo self (Transformation|GetActorLocation (Utilities|Array|Get(acopy) (Variables|Default|GetTargetPoints) (Variables|Default|GetIndexTargetPoints))) 0 5.0 false
        (:OnSuccess
          (Utilities|FlowControl|Delay 1.0)
          (CallFunction|NextPoint))))))

(event Custom|Explorar
  (CallFunction|SetIASpeed 0)
  (AI|AIMoveTo self (.RandomLocation (AI|Navigation|GetRandomReachablePointinRadius (Transformation|GetActorLocation) 5e+02 0 0)) 0 5.0 false))

(event EventBeginPlay
  (switch Utilities|FlowControl|Switch|Switchon (Variables|Default|GetIAStates)
    (:NewEnumerator0
      (CallFunction|Patrol))))

(fn ConstructionScript)