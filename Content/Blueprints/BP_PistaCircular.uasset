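; BP_PistaCircular is a circular track whose Plataforma component tilts slightly with the player's movement.
; BeginPlay caches the BP_Personaje player character.
; Every Tick, regardless of overlap, it converts player velocity into platform local space, normalizes it, derives clamped pitch and roll, and eases toward that relative rotation with RInterpTo, keeping yaw at zero.
; Leveling the platform once the player has the key is unfinished and never runs.
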(event EventBeginPlay
  ;[0.0471 0.15 0.0781 0.5] Generamos referencia del character
  (bind _asbp_personaje (Utilities|Casting|CastToBP_Personaje (Game|GetPlayerCharacter 0)))
  (Variables|Default|SetJugador _asbp_personaje))

(event Collision|EventActorBeginOverlap
  (params (OtherActor :type Actor%20Object%20Reference)))

(event EventTick
  (params (DeltaSeconds :type Float%20%28single-precision%29))
  (bind _jugador (Variables|Default|GetJugador))
  (bind _plataforma (Variables|Default|GetPlataforma))
  (bind _returnvalue (Transformation|GetVelocity _jugador))
  (bind _returnvalue_2 (Transformation|GetWorldTransform _plataforma))
  (bind _returnvalue_3 (Math|Transform|InverseTransformDirection _returnvalue_2 _returnvalue))
  (bind _returnvalue_4 (Math|Vector|Normalize _returnvalue_3))
  (bind (_x _y) (Math|Vector|BreakVector _returnvalue_4))
  ;[0.04393 0.15 0.07045 0.5] Actualizamos la rotacion de la plataforma en función de la velocidad del player. La Z siempre es cero.
  (Transformation|SetRelativeRotation (Variables|Default|GetPlataforma) (Math|Interpolation|RInterpTo (.Rotation (Math|Transform|BreakTransform (Transformation|GetRelativeTransform (Variables|Default|GetPlataforma)))) (Math|Rotator|MakeRotator (Math|Float|Clamp(Float) (* _y 5.0) -2.0 2.0) (Math|Float|Clamp(Float) (* _x -5.0) -2.0 2.0) 0.0) DeltaSeconds 5.0) false false))

(fn ConstructionScript)