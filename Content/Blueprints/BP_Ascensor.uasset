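; BP_Ascensor is an elevator that raises its Cylinder when a BPI_Personaje actor overlaps its sphere or PlayElevator is called.
; A Timeline lerps the cylinder's world Z toward FMovElevator, keeping X and Y.
; HasKey on GI_GameInstance gates the target: a held key is consumed and the current height used.
; Without a key, the elevator still runs, but FMovElevator is first overwritten with a fixed height.
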(event OnComponentBeginOverlap(SphereCollision)
  (params (OverlappedComponent :type Primitive%20Component%20Object%20Reference) (OtherActor :type Actor%20Object%20Reference) (OtherComp :type Primitive%20Component%20Object%20Reference) (OtherBodyIndex :type Integer) (bFromSweep :type Boolean) (SweepResult :type Hit%20Result%20Structure%20%28by%20ref%29))
  (bind _cylinder (Variables|Default|GetCylinder))
  (bind _returnvalue (Transformation|GetWorldTransform _cylinder))
  (bind _location (Math|Transform|BreakTransform _returnvalue))
  ;[0.02796 0.15 0.04791 0.5] Es un ascensor que a trasvés de una funcion que llama el character le pasa la altura final.
  ;;[0 0.15 0.05484 0.5] Cuando chocamos con player hacemos que se eleve el ascendor.
  (if (Utilities|DoesObjectImplementInterface OtherActor "/Game/Blueprints/BPI_Personaje.BPI_Personaje_C")
    (if (Variables|/Game/Blueprints/GI_GameInstance.GI_GameInstance_C|GetbHasKey (Variables|Default|GetInstance_GI))
      (Variables|/Game/Blueprints/GI_GameInstance.GI_GameInstance_C|SetbHasKey (Variables|Default|GetInstance_GI) false)
      (bind _newtrack_0 (Timeline|Timeline PlayFromStart)
        (:Update
          (Transformation|SetWorldLocation (Variables|Default|GetCylinder) (Math|Vector|MakeVector (.x (Math|Vector|Lerp(Vector) (Math|Vector|MakeVector (.x _location) (.y _location) 0.0) (Math|Vector|MakeVector (.x _location) (.y _location) (Variables|Default|GetfMovElevator)) _newtrack_0)) (.y (Math|Vector|Lerp(Vector) (Math|Vector|MakeVector (.x _location) (.y _location) 0.0) (Math|Vector|MakeVector (.x _location) (.y _location) (Variables|Default|GetfMovElevator)) _newtrack_0)) (.z (Math|Vector|Lerp(Vector) (Math|Vector|MakeVector (.x _location) (.y _location) 0.0) (Math|Vector|MakeVector (.x _location) (.y _location) (Variables|Default|GetfMovElevator)) _newtrack_0))) false false)))
      (else
        (Variables|Default|SetfMovElevator 3e+03)
        (Timeline|Timeline PlayFromStart)))))

(event EventBeginPlay
  ;[0 0.15 0.03849 0.5] Casteamos el Game Instance para acceder a HasKey
  (bind _asgi_game_instance (Utilities|Casting|CastToGI_GameInstance (Game|GetGameInstance)))
  (Variables|Default|SetInstance_GI _asgi_game_instance))

(event EventPlayElevator
  (bind _cylinder (Variables|Default|GetCylinder))
  (bind _returnvalue (Transformation|GetWorldTransform _cylinder))
  (bind _location (Math|Transform|BreakTransform _returnvalue))
  ;[0.02796 0.15 0.04791 0.5] Es un ascensor que a trasvés de una funcion que llama el character le pasa la altura final.
  (if (Variables|/Game/Blueprints/GI_GameInstance.GI_GameInstance_C|GetbHasKey (Variables|Default|GetInstance_GI))
    (Variables|/Game/Blueprints/GI_GameInstance.GI_GameInstance_C|SetbHasKey (Variables|Default|GetInstance_GI) false)
    (bind _newtrack_0 (Timeline|Timeline PlayFromStart)
      (:Update
        (Transformation|SetWorldLocation (Variables|Default|GetCylinder) (Math|Vector|MakeVector (.x (Math|Vector|Lerp(Vector) (Math|Vector|MakeVector (.x _location) (.y _location) 0.0) (Math|Vector|MakeVector (.x _location) (.y _location) (Variables|Default|GetfMovElevator)) _newtrack_0)) (.y (Math|Vector|Lerp(Vector) (Math|Vector|MakeVector (.x _location) (.y _location) 0.0) (Math|Vector|MakeVector (.x _location) (.y _location) (Variables|Default|GetfMovElevator)) _newtrack_0)) (.z (Math|Vector|Lerp(Vector) (Math|Vector|MakeVector (.x _location) (.y _location) 0.0) (Math|Vector|MakeVector (.x _location) (.y _location) (Variables|Default|GetfMovElevator)) _newtrack_0))) false false)))
    (else
      (Variables|Default|SetfMovElevator 3e+03)
      (Timeline|Timeline PlayFromStart))))

(fn ConstructionScript)